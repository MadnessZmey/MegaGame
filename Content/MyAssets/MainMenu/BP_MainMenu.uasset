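; BP_MainMenu is a 3D main menu actor that hands the player's view over to other linked menu actors.
; At BeginPlay it binds to its WD_3DMenu widget's transition event and turns off its own collision.
; The event's index selects an entry in LinkedMenu; the transition disables this actor's collision, enables the target's and eases the view target to it with a timed blend.
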(event Custom|TransitionTo
  (params (NewMenu :type BP%20Main%20Menu%20Object%20Reference))
  (Collision|SetActorEnableCollision false)
  (Collision|SetActorEnableCollision NewMenu true)
  (Game|Player|SetViewTargetwithBlend (Game|GetPlayerController 0) NewMenu 2.0 "VTBlend_EaseInOut" 2.0 false))

(event Custom|OnTransitionBetweenMenu
  (params (MenuIndex :type Integer))
  (if (Utilities|Array|IsValidIndex (Variables|Default|GetLinkedMenu) MenuIndex)
    (CallFunction|Transitionto (Utilities|Array|Get(acopy) (Variables|Default|GetLinkedMenu) MenuIndex))))

(event EventBeginPlay
  (bind _aswd_3dmenu (Utilities|Casting|CastToWD_3DMenu (UserInterface|GetUserWidgetObject (Variables|Default|GetWidget_MainMenu))))
  (EventDispatchers|BindEventtoEDTransitiontoLinkedMenu _aswd_3dmenu (delegate Custom|OnTransitionBetweenMenu))
  (Collision|SetActorEnableCollision false))

(fn ConstructionScript)