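; BP_BigBotSpawn is a trigger-driven spawner that introduces an AI bot with a brief player freeze.
; The first Box1 overlap clears CheckBot, waits briefly, then spawns PawnClass at a random point inside the BoxSize-driven Box, with explosion effect and sound.
; It then removes all widgets, disables BP_BigPlayerCharacter input briefly, re-possesses it and calls OnWidget.
; The timer-based SpawnEnemy path is unconnected and unfinished.
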(event OnComponentBeginOverlap(Box1)
  (params (OverlappedComponent :type Primitive%20Component%20Object%20Reference) (OtherActor :type Actor%20Object%20Reference) (OtherComp :type Primitive%20Component%20Object%20Reference) (OtherBodyIndex :type Integer) (bFromSweep :type Boolean) (SweepResult :type Hit%20Result%20Structure%20%28by%20ref%29))
  (bind _box (Variables|Default|GetBox))
  (bind _returnvalue (Transformation|GetWorldLocation _box))
  (bind _returnvalue_2 (Components|Box|GetScaledBoxExtent _box))
  (bind _returnvalue_3 (Math|Random|RandomPointinBoundingBox _returnvalue _returnvalue_2))
  (if (Variables|Default|GetCheckBot)
    (Variables|Default|SetCheckBot false)
    (Utilities|FlowControl|Delay 0.5)
    (bind _returnvalue_4 (AI|SpawnAIFromClass (Variables|Default|GetPawn%20Class) 0 (Math|Vector|MakeVector (.x _returnvalue_3) (.y _returnvalue_3) (+ (.z _returnvalue_3) 2e+01)) "0, 0, 0" false 0))
    (Effects|SpawnEmitteratLocation "/Game/Assets/SciFiWeapLight/FX/Particles/P_RocketLauncher_Explosion_Dark.P_RocketLauncher_Explosion_Dark" (Pawn|GetNavAgentLocation _returnvalue_4) "0, 0, 0" "3.000000,3.000000,3.000000")
    (Audio|PlaySoundatLocation "/Game/Assets/SciFiWeapLight/Sound/RocketLauncher/Wavs/RL_Explosion05.RL_Explosion05" (Pawn|GetNavAgentLocation _returnvalue_4) "0, 0, 0" 0.4 1.0 0.0 0 0 0)
    (Viewport|RemoveAllWidgets)
    (bind _returnvalue_5 (Actor|GetActorOfClass "/Game/MyAssets/BigPlayer/BP_BigPlayerCharacter.BP_BigPlayerCharacter_C"))
    (bind _output_get (Variables|Default|SetPerson _returnvalue_5))
    (Input|DisableInput _output_get 0)
    (Utilities|FlowControl|Delay 1.5)
    (Input|EnableInput (Variables|Default|GetPerson) 0)
    (Pawn|Possess (Game|GetPlayerController 0) (Variables|Default|GetPerson))
    (Default|OnWidget (Variables|Default|GetPerson))))

(event Custom|SpawnEnemy
  (bind _outactors (Actor|GetAllActorsOfClass "/Game/Blueprints/Enemy/BP_Ai_Master.BP_Ai_Master_C"))
  (if (< (Utilities|Array|Length _outactors) 3)
    _))

(fn ConstructionScript
  (Components|Box|SetBoxExtent (Variables|Default|GetBox) (Variables|Default|GetBoxSize) true))