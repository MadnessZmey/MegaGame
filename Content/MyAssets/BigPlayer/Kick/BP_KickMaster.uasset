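; Base kick Blueprint for the player character (BP_BigPlayerCharacter) that plays a kick montage and deals melee damage.
; The construction script loads damage, cooldown and montage from a DT_Kick row.
; Kick enables capsule collision, plays the montage on the player, then disables collision after the montage's duration.
; Capsule overlap sends a TakingDamage message with the hit bone, with a flag limiting damage to one hit per kick.
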(event OnComponentBeginOverlap(Capsule)
  (params (OverlappedComponent :type Primitive%20Component%20Object%20Reference) (OtherActor :type Actor%20Object%20Reference) (OtherComp :type Primitive%20Component%20Object%20Reference) (OtherBodyIndex :type Integer) (bFromSweep :type Boolean) (SweepResult :type Hit%20Result%20Structure%20%28by%20ref%29))
  (bind (_bblockinghit _binitialoverlap _time _distance _location _impactpoint _normal _impactnormal _physmat _hitactor _hitcomponent _hitbonename) (Collision|BreakHitResult SweepResult))
  ;[1 1 1] Срабатывает, когда касается меша игрока, поправить
  (if (and (Variables|Default|GetGetKickDelay) (!= OtherActor (Variables|Default|GetCharRef)))
    (Class|BPITakeDamage|TakingDamage(Message) _hitactor _hitbonename (Variables|Default|GetDamageKick) (Game|GetInstigator))
    (Variables|Default|SetGetKickDelay false)))

(event Custom|Kick
  (bind _charref (Variables|Default|GetCharRef))
  (bind _kickmontage (Variables|Default|GetKickMontage))
  (Variables|Default|SetGetKickDelay true)
  (Collision|SetCollisionEnabled (Variables|Default|GetCapsule) "QueryAndPhysics")
  (if (not (Animation|Montage|MontageIsPlaying (Components|SkeletalMesh|GetAnimInstance (Variables|/Script/Engine.Character|GetMesh _charref)) _kickmontage))
    (bind _returnvalue (Animation|PlayAnimMontage _charref _kickmontage 1.0 "None"))
    (bind _output_get (Variables|Default|SetDelayMontage _returnvalue))
    (Utilities|FlowControl|Delay _output_get)
    (Collision|SetCollisionEnabled (Variables|Default|GetCapsule) "NoCollision")))

(event EventBeginPlay
  ;[1 1 1] Каст на персонажа
  (bind _asbp_big_player_character (Utilities|Casting|CastToBP_BigPlayerCharacter (Game|Player|GetPlayerPawn 0)))
  (Variables|Default|SetCharRef _asbp_big_player_character))

(fn ConstructionScript
  (bind _returnvalue (Utilities|GetDataTableRow "/Game/MyAssets/BigPlayer/Kick/DT_Kick.DT_Kick" (Variables|Default|GetKickRownName))
    (:then
      (bind _output_get (Variables|Default|SetKickData _returnvalue))
      (Variables|Default|SetDamageKick (.DamageKick (Utilities|Struct|BreakStruct_Kick _output_get)))
      (Variables|Default|SetCooldownKick (.CooldownKick (Utilities|Struct|BreakStruct_Kick _output_get)))
      (Variables|Default|SetKickMontage (.KickMontage (Utilities|Struct|BreakStruct_Kick _output_get))))))