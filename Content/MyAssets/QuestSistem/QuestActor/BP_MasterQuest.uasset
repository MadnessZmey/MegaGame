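; BP_MasterQuest is a quest Blueprint, apparently the base for quests, that tracks active sub-goals from its QuestInfo data.
; SetapStartingGoals copies the starting indices into the current ones and calls UpdateSubGoals to rebuild CurrentGoal.
; GoToNextSubGoal replaces the current indices with the highest plus one and reports success.
; UpdateSubGoals always reads StartingSubGoalIndices, so advancing leaves CurrentGoal on the starting sub-goals.
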(event EventBeginPlay)

(event Collision|EventActorBeginOverlap
  (params (OtherActor :type Actor%20Object%20Reference)))

(event EventTick
  (params (DeltaSeconds :type Float%20%28single-precision%29)))

(fn ConstructionScript)

(fn UpdateSubGoals
  (Utilities|Array|Clear (Variables|DoNotTouch!|GetCurrentGoal))
  (for (_ _array_index) (Variables|QuestInformation|GetStartingSubGoalIndices)
    (Utilities|Array|Add (Variables|DoNotTouch!|GetCurrentGoal) (Utilities|Array|Get(acopy) (.SabGoal (Utilities|Struct|BreakStruct_QuestInfo (Variables|QuestInformation|GetQuestInfo))) _array_index)))
  (return))

(fn SetapStartingGoals
  (Utilities|Array|Clear (Variables|DoNotTouch!|GetCurentGoalIndices))
  (Variables|DoNotTouch!|SetCurentGoalIndices (Variables|QuestInformation|GetStartingSubGoalIndices))
  (CallFunction|UpdateSubGoals)
  (return))

(fn GotoNextSubGoal
  (bind _curentgoalindices (Variables|DoNotTouch!|GetCurentGoalIndices))
  (bind _curentgoalindices_2 (Variables|DoNotTouch!|GetCurentGoalIndices))
  (bind _maxvalue (Math|Integer|MaxOfIntArray _curentgoalindices))
  (bind _returnvalue (+ _maxvalue 1))
  (if (<= _returnvalue (Utilities|Array|Length (.SabGoal (Utilities|Struct|BreakStruct_QuestInfo (Variables|QuestInformation|GetQuestInfo)))))
    (LocalVariables|SetL_NextIndex _returnvalue)
    (Utilities|Array|Clear _curentgoalindices_2)
    (Utilities|Array|Add _curentgoalindices_2 (LocalVariables|GetL_NextIndex))
    (CallFunction|UpdateSubGoals)
    (return true)
    (else
      (return false))))