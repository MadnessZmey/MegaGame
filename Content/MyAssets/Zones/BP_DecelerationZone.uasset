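; BP_DecelerationZone is a zone actor that changes the speed of AI characters, AI bullets and projectiles inside its Cube volume.
; On begin overlap it casts the actor, setting a deceleration flag and speed multiplier on AI or calling SwitchSpeed on bullets and projectiles.
; End overlap restores normal speed.
; Damage timer and timeline-driven cube resizing nodes exist but are never executed, and the DamageZone event is empty.
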(event OnComponentBeginOverlap(Cube)
  (params (OverlappedComponent :type Primitive%20Component%20Object%20Reference) (OtherActor :type Actor%20Object%20Reference) (OtherComp :type Primitive%20Component%20Object%20Reference) (OtherBodyIndex :type Integer) (bFromSweep :type Boolean) (SweepResult :type Hit%20Result%20Structure%20%28by%20ref%29))
  ;[1 1 1] Пересечение коллизи
  (Utilities|FlowControl|Sequence
    (:then_0
      ;[1 1 1] Каст на персонажа
      (bind _asbp_ai_master (Utilities|Casting|CastToBP_Ai_Master OtherActor))
      (Variables|/Game/Blueprints/Enemy/BP_Ai_Master.BP_Ai_Master_C|SetIsDeceleration? _asbp_ai_master true)
      (Variables|/Game/Blueprints/Enemy/BP_Ai_Master.BP_Ai_Master_C|SetSpeedMultiplierAI _asbp_ai_master (Variables|Default|GetSpeedMultiplier)))
    (:then_1
      (bind _asbp_ai_bullet (Utilities|Casting|CastToBP_Ai_Bullet OtherActor))
      (Default|SwitchSpeed _asbp_ai_bullet (Variables|Default|GetSpeedMultiplier)))
    (:then_2
      (bind _asbp_master_projectile (Utilities|Casting|CastToBP_Master_Projectile OtherActor))
      (Default|SwitchSpeed _asbp_master_projectile (Variables|Default|GetSpeedMultiplier)))))

(event OnComponentEndOverlap(Cube)
  (params (OverlappedComponent :type Primitive%20Component%20Object%20Reference) (OtherActor :type Actor%20Object%20Reference) (OtherComp :type Primitive%20Component%20Object%20Reference) (OtherBodyIndex :type Integer))
  ;[1 1 1] Пересечение коллизи
  (Utilities|FlowControl|Sequence
    (:then_0
      ;[1 1 1] Каст на персонажа
      (bind _asbp_ai_master (Utilities|Casting|CastToBP_Ai_Master OtherActor))
      (Variables|/Game/Blueprints/Enemy/BP_Ai_Master.BP_Ai_Master_C|SetIsDeceleration? _asbp_ai_master false)
      (Variables|/Game/Blueprints/Enemy/BP_Ai_Master.BP_Ai_Master_C|SetSpeedMultiplierAI _asbp_ai_master (Variables|Default|GetSpeedNormal)))
    (:then_1
      (bind _asbp_ai_bullet (Utilities|Casting|CastToBP_Ai_Bullet OtherActor))
      (Default|SwitchSpeed _asbp_ai_bullet (Variables|Default|GetSpeedNormal)))
    (:then_2
      (bind _asbp_master_projectile (Utilities|Casting|CastToBP_Master_Projectile OtherActor))
      (Default|SwitchSpeed _asbp_master_projectile (Variables|Default|GetSpeedNormal)))))

(event Custom|DamageZone
  (if (Variables|Default|GetDamageOn?)
    _))

(event EventBeginPlay)

(fn ConstructionScript)