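; BP_DamageZone is a zone that marks player characters while they overlap its Cube volume.
; Shortly after BeginPlay, the Size_1 timeline rescales the cube along X while holding Y and Z fixed.
; Overlap begin sets Outside to true on BP_Master_PlayerCharacter and overlap end clears it.
; The DamageZone event is empty, and the looping timer, damage message and second resize timeline are disconnected.
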(event OnComponentBeginOverlap(Cube)
  (params (OverlappedComponent :type Primitive%20Component%20Object%20Reference) (OtherActor :type Actor%20Object%20Reference) (OtherComp :type Primitive%20Component%20Object%20Reference) (OtherBodyIndex :type Integer) (bFromSweep :type Boolean) (SweepResult :type Hit%20Result%20Structure%20%28by%20ref%29))
  ;[1 1 1] Пересечение коллизи
  ;[1 1 1] Каст на персонажа
  (bind _asbp_master_character (Utilities|Casting|CastToBP_Master_PlayerCharacter OtherActor))
  (Variables|/Game/Blueprints/Player/BP_Master_PlayerCharacter.BP_Master_PlayerCharacter_C|SetOutside _asbp_master_character true))

(event OnComponentEndOverlap(Cube)
  (params (OverlappedComponent :type Primitive%20Component%20Object%20Reference) (OtherActor :type Actor%20Object%20Reference) (OtherComp :type Primitive%20Component%20Object%20Reference) (OtherBodyIndex :type Integer))
  ;[1 1 1] Пересечение коллизи
  ;[1 1 1] Каст на персонажа
  (bind _asbp_master_character (Utilities|Casting|CastToBP_Master_PlayerCharacter OtherActor))
  (Variables|/Game/Blueprints/Player/BP_Master_PlayerCharacter.BP_Master_PlayerCharacter_C|SetOutside _asbp_master_character false))

(event Custom|DamageZone
  (if (Variables|Default|GetDamageOn?)
    _))

(event EventBeginPlay
  (Utilities|FlowControl|Delay 0.2)
  (bind _t_zone1 (Timeline|Size_1 Play)
    (:Update
      (Transformation|SetWorldScale3D (Variables|Default|GetCube) (Math|Vector|MakeVector (.x (Math|Conversions|ToVector(Float) _t_zone1)) 6e+01 2e+01)))))

(fn ConstructionScript)