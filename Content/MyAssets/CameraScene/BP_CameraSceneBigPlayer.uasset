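; End-scene trigger actor for BP_BigPlayerCharacter that switches to its own camera view, plays a barrage of explosions and returns to the main menu.
; Box overlap hides the text, then after a short delay blends the view to this actor and disables the character's input.
; A looping timer spawns explosion effects and sounds at random points in Box1 until a counter limit, then opens Map_MainMenu.
; The branch that blends back to the player is unconnected.
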(event OnComponentEndOverlap(Box)
  (params (OverlappedComponent :type Primitive%20Component%20Object%20Reference) (OtherActor :type Actor%20Object%20Reference) (OtherComp :type Primitive%20Component%20Object%20Reference) (OtherBodyIndex :type Integer))
  (Utilities|Casting|CastToBP_BigPlayerCharacter OtherActor)
  (Input|DisableInput (Game|GetPlayerController 0))
  (Rendering|SetVisibility (Variables|Default|GetTextRender) true false))

(event OnComponentBeginOverlap(Box)
  (params (OverlappedComponent :type Primitive%20Component%20Object%20Reference) (OtherActor :type Actor%20Object%20Reference) (OtherComp :type Primitive%20Component%20Object%20Reference) (OtherBodyIndex :type Integer) (bFromSweep :type Boolean) (SweepResult :type Hit%20Result%20Structure%20%28by%20ref%29))
  (Utilities|FlowControl|Sequence
    (:then_0
      ;[1 1 1] Каст на персонажа
      (bind _asbp_big_player_character (Utilities|Casting|CastToBP_BigPlayerCharacter (Game|GetPlayerCharacter 0)))
      (Variables|Default|SetCharRefBig _asbp_big_player_character))
    (:then_1
      (Utilities|Casting|CastToBP_BigPlayerCharacter OtherActor)
      (Input|EnableInput (Game|GetPlayerController 0))
      (Rendering|SetVisibility (Variables|Default|GetTextRender) false false)
      (Utilities|FlowControl|Delay 0.5)
      (Variables|Default|SetCameraSwitch true)
      (Game|Player|SetViewTargetwithBlend (Game|GetPlayerController 0) self (Variables|Default|GetDelayCameraBlend) "VTBlend_Linear" 0.0 false)
      (Input|DisableInput (Variables|Default|GetCharRefBig) 0)
      (Utilities|FlowControl|Delay 0.2)
      (Rendering|SetVisibility (Variables|Default|GetTextRender) true false)
      (Utilities|FlowControl|Delay (Variables|Default|GetDelayCameraBlend))
      (Variables|Default|SetDelayCamera false)
      (Utilities|FlowControl|Delay 2.5)
      (Utilities|Time|SetTimerbyEvent (delegate Custom|Explotions) 0.4 true))))

(event Custom|Explotions
  (bind _box1 (Variables|Default|GetBox1))
  (bind _returnvalue (Transformation|GetWorldLocation _box1))
  (bind _returnvalue_2 (Components|Box|GetScaledBoxExtent _box1))
  (bind _returnvalue_3 (Math|Random|RandomPointinBoundingBox _returnvalue _returnvalue_2))
  (if (< (Variables|Default|GetNumberOfExplosions) 10)
    (bind _result (Math|Integer|IncrementInt (Variables|Default|GetNumberOfExplosions))
      (:%20%20
        (Variables|Default|SetNumberOfExplosions _result)
        (Effects|SpawnEmitteratLocation "/Game/Assets/SciFiWeapLight/FX/Particles/P_RocketLauncher_Explosion_Dark.P_RocketLauncher_Explosion_Dark" (Math|Vector|MakeVector (.x _returnvalue_3) (.y _returnvalue_3) (+ (.z _returnvalue_3) 2e+01)) "0, 0, 0" "3.000000,3.000000,3.000000")
        (Audio|PlaySoundatLocation "/Game/Assets/SciFiWeapLight/Sound/GrenadeLauncher/Wavs/GL_Explosion02.GL_Explosion02" "0, 0, 0" "0, 0, 0" 0.4 1.0 0.0 0 0 0)))
    (else
      (Utilities|FlowControl|Delay 1.5)
      (Game|OpenLevel(byName) "Map_MainMenu"))))

(event EventBeginPlay
  ;[1 1 1] Каст на персонажа
  (bind _asbp_big_player_character (Utilities|Casting|CastToBP_BigPlayerCharacter (Game|GetPlayerCharacter 0)))
  (Variables|Default|SetCharRefBig _asbp_big_player_character))

(event Input|ActionEvents|InputActionInteract
  (params (Key :type Key%20Structure :default "None")))

(fn ConstructionScript)