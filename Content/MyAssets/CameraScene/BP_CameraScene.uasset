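; Interactable camera actor that lets the player switch between their character's view and this scene's camera.
; Entering its box trigger enables input on the actor and shows a text prompt; leaving reverses both.
; Interact toggles a blended view-target change, hiding the prompt and disabling character input while viewing the scene.
; The DelayCamera flag flips only after the blend delay, so the toggle direction changes once the transition finishes.
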(event OnComponentEndOverlap(Box)
  (params (OverlappedComponent :type Primitive%20Component%20Object%20Reference) (OtherActor :type Actor%20Object%20Reference) (OtherComp :type Primitive%20Component%20Object%20Reference) (OtherBodyIndex :type Integer))
  (Utilities|Casting|CastToBP_Master_PlayerCharacter OtherActor)
  (Input|DisableInput (Game|GetPlayerController 0))
  (Rendering|SetVisibility (Variables|Default|GetTextRender) false false))

(event OnComponentBeginOverlap(Box)
  (params (OverlappedComponent :type Primitive%20Component%20Object%20Reference) (OtherActor :type Actor%20Object%20Reference) (OtherComp :type Primitive%20Component%20Object%20Reference) (OtherBodyIndex :type Integer) (bFromSweep :type Boolean) (SweepResult :type Hit%20Result%20Structure%20%28by%20ref%29))
  (Utilities|FlowControl|Sequence
    (:then_0
      ;[1 1 1] Каст на персонажа
      (bind _asbp_master_character (Utilities|Casting|CastToBP_Master_PlayerCharacter (Game|GetPlayerCharacter 0)))
      (Variables|Default|SetCharRef _asbp_master_character))
    (:then_1
      (Utilities|Casting|CastToBP_Master_PlayerCharacter OtherActor)
      (Input|EnableInput (Game|GetPlayerController 0))
      (Rendering|SetVisibility (Variables|Default|GetTextRender) true false))))

(event EventBeginPlay
  ;[1 1 1] Каст на персонажа
  (bind _asbp_master_character (Utilities|Casting|CastToBP_Master_PlayerCharacter (Game|GetPlayerCharacter 0)))
  (Variables|Default|SetCharRef _asbp_master_character))

(event Input|ActionEvents|InputActionInteract
  (params (Key :type Key%20Structure))
  (bind _charref (Variables|Default|GetCharRef))
  (bind _delaycamerablend (Variables|Default|GetDelayCameraBlend))
  (bind _textrender (Variables|Default|GetTextRender))
  (bind _delaycamerablend_2 (Variables|Default|GetDelayCameraBlend))
  (:Pressed
    (if (Variables|Default|GetDelayCamera)
      (Variables|Default|SetCameraSwitch true)
      (Game|Player|SetViewTargetwithBlend (Game|GetPlayerController 0) self _delaycamerablend "VTBlend_Linear" 0.0 false)
      (Rendering|SetVisibility _textrender false false)
      (Input|DisableInput _charref 0)
      (Utilities|FlowControl|Delay _delaycamerablend_2)
      (Variables|Default|SetDelayCamera false)
      (else
        (Variables|Default|SetCameraSwitch false)
        (Game|Player|SetViewTargetwithBlend (Game|GetPlayerController 0) _charref _delaycamerablend "VTBlend_Linear" 0.0 false)
        (Rendering|SetVisibility _textrender true false)
        (Input|EnableInput _charref 0)
        (Utilities|FlowControl|Delay _delaycamerablend_2)
        (Variables|Default|SetDelayCamera true)))))

(fn ConstructionScript)