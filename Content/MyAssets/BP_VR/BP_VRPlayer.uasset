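; VR player that enables stereo with floor-level tracking and makes a detached skeletal body mesh follow the headset camera.
; Each tick, camera movement or yaw change beyond thresholds sets a new offset body target, movement speed and direction.
; Below the thresholds, the body interpolates toward that target at that speed.
; Body height tracks camera height minus player height every tick for IK, independent of the smoothing.
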(event EventBeginPlay
  (Development|ExecuteConsoleCommand "stereo on" 0)
  (Class|HeadMountedDisplayFunctionLibrary|SetTrackingOrigin "Floor"))

(event Collision|EventActorBeginOverlap
  (params (OtherActor :type Actor%20Object%20Reference)))

(event EventTick
  (params (DeltaSeconds :type Float%20%28single-precision%29))
  (CallFunction|CalculateMovement))

(fn ConstructionScript
  (Transformation|DetachFromComponent (Variables|Default|GetSkeletalMesh) "KeepRelative" "KeepRelative" "KeepRelative" true))

(fn CalculateMovement
  (bind (_location _rotation) (CallFunction|GetBodyOffset))
  (bind _camera (Variables|Default|GetCamera))
  (bind _returnvalue (Transformation|GetWorldTransform _camera))
  (bind _output_get (LocalVariables|SetCurrent%20Camera%20Position (Math|Transform|MakeTransform (Math|Vector|MakeVector (.x (.location _returnvalue)) (.y (.location _returnvalue)) 0.0) (Math|Rotator|MakeRotator 0.0 0.0 (.yaw (.rotation _returnvalue))) "1,1,1")))
  (bind _distance_moved (CallFunction|GetDistanceMoved (.x (.location _output_get)) (.y (.location _output_get))))
  (LocalVariables|SetDistance%20Moved _distance_moved)
  (bind _distance_rotated (CallFunction|GetDistanceRotated (.rotation _output_get)))
  (LocalVariables|SetDistance%20Rotated _distance_rotated)
  (Utilities|FlowControl|Sequence
    (:then_0
      ;[1 1 1] Если порог достигнут, установка новой позиции, иначе интерполяция позиции
      (if (or (> (LocalVariables|GetDistance%20Moved) (Variables|Default|GetMovement%20Threshold)) (> (LocalVariables|GetDistance%20Rotated) (Variables|Default|GetRatation%20Threshold)))
        (Variables|Default|SetBody%20Target%20Position (Math|Transform|MakeTransform _location _rotation "1,1,1"))
        (Variables|Default|SetMovement%20Direction (Utilities|GetDirection (LocalVariables|GetCurrent%20Camera%20Position)))
        (Variables|Default|SetLast%20Camera%20Position (LocalVariables|GetCurrent%20Camera%20Position))
        (Variables|Default|SetMovement%20Speed (/ (/ (+ (LocalVariables|GetDistance%20Moved) (LocalVariables|GetDistance%20Rotated)) 2e+03) (Utilities|Time|GetWorldDeltaSeconds)))
        (elif (== (Variables|Default|GetBody%20Current%20Position) (Variables|Default|GetBody%20Target%20Position))
          (Variables|Default|SetMovement%20Speed 0.0)
          (Variables|Default|SetMovement%20Direction 0.0)
          (Variables|Default|SetAlpha 0.0)
          (else
            (Variables|Default|SetAlpha (Math|Interpolation|FInterptoConstant (Variables|Default|GetAlpha) 1.0 (Utilities|Time|GetWorldDeltaSeconds) (Variables|Default|GetMovement%20Speed)))
            (bind _output_get_2 (Variables|Default|SetBody%20Current%20Position (Math|Transform|Lerp(Transform) (Variables|Default|GetBody%20Current%20Position) (Variables|Default|GetBody%20Target%20Position) (Variables|Default|GetAlpha))))
            (Transformation|SetWorldLocationAndRotation (Variables|Default|GetSkeletalMesh) (.location _output_get_2) (.rotation _output_get_2) false false)))))
    (:then_1
      ;;[1 1 1] Только Z для IK
      (Transformation|SetWorldLocationAndRotation (Variables|Default|GetSkeletalMesh) (Math|Vector|MakeVector (.x (.location (Variables|Default|GetBody%20Current%20Position))) (.y (.location (Variables|Default|GetBody%20Current%20Position))) (.z (.Location (CallFunction|GetBodyOffset)))) (.rotation (Variables|Default|GetBody%20Current%20Position)) false false))))

(fn GetDistanceMoved
  (params (Current%20X :type Float%20%28single-precision%29) (Current%20Y :type Float%20%28single-precision%29))
  (bind _last_camera_position (Variables|Default|GetLast%20Camera%20Position))
  (return (Math|Vector|Distance(Vector) (Math|Vector|MakeVector Current%20X Current%20Y 0.0) (Math|Vector|MakeVector (.x (.location _last_camera_position)) (.y (.location _last_camera_position)) 0.0))))

(fn GetDistanceRotated
  (params (Current%20Roation :type Rotator))
  (return (Math|Float|Absolute(Float) (- (.yaw Current%20Roation) (.yaw (.rotation (Variables|Default|GetLast%20Camera%20Position)))))))

(fn GetBodyOffset
  (bind _camera (Variables|Default|GetCamera))
  (bind _returnvalue (Transformation|GetWorldTransform _camera))
  (bind _returnvalue_2 (- (.yaw (.rotation _returnvalue)) 9e+01))
  (bind _returnvalue_3 (Math|Rotator|MakeRotator 0.0 0.0 _returnvalue_2))
  (bind _returnvalue_4 (Math|Vector|GetRightVector _returnvalue_3))
  (bind _returnvalue_5 (* _returnvalue_4 -2e+01))
  (bind _returnvalue_6 (+ (.location _returnvalue) _returnvalue_5))
  (return (Math|Vector|MakeVector (.x _returnvalue_6) (.y _returnvalue_6) (- (.z _returnvalue_6) (Variables|Default|GetPlayer%20Height))) _returnvalue_3))