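; BP_CameraSwitch is an interactable that blends the player's view to its own camera and back.
; Overlapping its box with BP_PlayerCharacter enables input on the actor and shows a text prompt; leaving reverses both.
; Pressing E blends the view over two seconds, hiding the prompt and ignoring move and look input while switched away.
; DelayCamera picks the direction and flips after a matching delay, while CameraSwitch records the state.
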(event OnComponentEndOverlap(Box)
  (params (OverlappedComponent :type Primitive%20Component%20Object%20Reference) (OtherActor :type Actor%20Object%20Reference) (OtherComp :type Primitive%20Component%20Object%20Reference) (OtherBodyIndex :type Integer))
  (Utilities|Casting|CastToBP_PlayerCharacter OtherActor)
  (Input|DisableInput (Game|GetPlayerController 0))
  (Rendering|SetVisibility (Variables|Default|GetTextRender) false false))

(event OnComponentBeginOverlap(Box)
  (params (OverlappedComponent :type Primitive%20Component%20Object%20Reference) (OtherActor :type Actor%20Object%20Reference) (OtherComp :type Primitive%20Component%20Object%20Reference) (OtherBodyIndex :type Integer) (bFromSweep :type Boolean) (SweepResult :type Hit%20Result%20Structure%20%28by%20ref%29))
  (Utilities|Casting|CastToBP_PlayerCharacter OtherActor)
  (Input|EnableInput (Game|GetPlayerController 0))
  (Rendering|SetVisibility (Variables|Default|GetTextRender) true false))

(event Input|KeyboardEvents|E
  (params (Key :type Key%20Structure :default "None"))
  (bind _returnvalue (Game|GetPlayerController 0))
  (bind _returnvalue_2 (Game|GetPlayerController 0))
  (bind _textrender (Variables|Default|GetTextRender))
  (:Pressed
    (if (Variables|Default|GetDelayCamera)
      (Variables|Default|SetCameraSwitch true)
      (Game|Player|SetViewTargetwithBlend _returnvalue_2 self 2.0 "VTBlend_Linear" 0.0 false)
      (Input|SetIgnoreMoveInput _returnvalue_2 true)
      (Input|SetIgnoreLookInput _returnvalue_2 true)
      (Rendering|SetVisibility _textrender false false)
      (Utilities|FlowControl|Delay 2.0)
      (Variables|Default|SetDelayCamera false)
      (else
        (Variables|Default|SetCameraSwitch false)
        (bind _asbp_player_character (Utilities|Casting|CastToBP_PlayerCharacter (Game|GetPlayerCharacter 0)))
        (Game|Player|SetViewTargetwithBlend _returnvalue _asbp_player_character 2.0 "VTBlend_Linear" 0.0 false)
        (Input|ResetIgnoreMoveInput _returnvalue)
        (Input|ResetIgnoreLookInput _returnvalue)
        (Rendering|SetVisibility _textrender true false)
        (Utilities|FlowControl|Delay 2.0)
        (Variables|Default|SetDelayCamera true)))))

(fn ConstructionScript)