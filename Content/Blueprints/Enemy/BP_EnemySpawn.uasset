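; Enemy spawner actor that keeps the level stocked with BP_Ai_Master enemies at random points inside a box volume.
; A looping one-second timer spawns one enemy whenever fewer than five exist.
; The count covers the whole world through GetAllActorsOfClass, so multiple spawners share the same cap.
; The construction script sizes the box from BoxSize, and spawn points are picked within that extent around the root location.
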(event Custom|SpawnEnemy
  (bind _outactors (Actor|GetAllActorsOfClass "/Game/Blueprints/Enemy/BP_Ai_Master.BP_Ai_Master_C"))
  (if (< (Utilities|Array|Length _outactors) 5)
    (Game|SpawnActorfromClass "/Game/Blueprints/Enemy/BP_Ai_Master.BP_Ai_Master_C" (Math|Transform|MakeTransform (Math|Random|RandomPointinBoundingBox (Transformation|GetWorldLocation (Variables|Default|GetDefaultSceneRoot)) (Variables|/Script/Engine.BoxComponent|GetBoxExtent (Variables|Default|GetBox)))) "Undefined" 0 0)))

(event EventBeginPlay
  (Utilities|Time|SetTimerbyEvent (delegate Custom|SpawnEnemy) 1.0 true))

(fn ConstructionScript
  (Components|Box|SetBoxExtent (Variables|Default|GetBox) (Variables|Default|GetBoxSize) true))