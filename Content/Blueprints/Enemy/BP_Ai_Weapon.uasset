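; BP_Ai_Weapon is an AI weapon that fires automatically while its Firing event is toggled on.
; Firing runs a self-repeating loop on a short fixed Delay, with a FireDelay flag blocking overlapping shots.
; Each shot spawns a BP_Ai_Bullet at the WeaponMesh Muzzle socket and plays the ImpulsGun montage on that mesh.
; BeginPlay only casts AiMasterRef to BP_Ai_Master, with nothing following the cast.
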(event Custom|Firing
  (params (Toggle :type Boolean))
  (bind _output_get (Variables|Default|SetCanFire Toggle))
  (if _output_get
    (if (and (Variables|Default|GetCanFire) (not (Variables|Default|GetFireDelay))) :!label _label
      (Variables|Default|SetFireDelay true)
      (CallFunction|SpawnProjectile)
      (Utilities|FlowControl|Delay 0.2)
      (Variables|Default|SetFireDelay false)
      (goto _label))))

(event EventBeginPlay
  (Utilities|Casting|CastToBP_Ai_Master (Variables|Default|GetAiMasterRef)))

(fn ConstructionScript)

(fn SpawnProjectile
  (Game|SpawnActorfromClass "/Game/Blueprints/Enemy/BP_Ai_Bullet.BP_Ai_Bullet_C" (Transformation|GetSocketTransform (Variables|Default|GetWeaponMesh) "Muzzle" "RTS_World") "Undefined" 0 0)
  (Animation|Montage|MontagePlay (Components|SkeletalMesh|GetAnimInstance (Variables|Default|GetWeaponMesh)) "/Game/Anim/Weapon/ImpulsGun_Montage.ImpulsGun_Montage" 1.0 "MontageLength" 0.0 true))