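; BP_Ai_Bullet is an enemy AI projectile that flies along its sphere's forward vector and is destroyed on hit.
; BeginPlay sets its velocity from speed and a multiplier, and SwitchSpeed recomputes it at runtime.
; Targets implementing BPI_TakeDamage receive fixed damage with bone name and instigator.
; Other surfaces get an impact particle, attached bullet-hole decal and sound, plus a velocity-scaled impulse when simulating physics.
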(event Custom|SwitchSpeed
  (params (SpeedMultiplier :type Float%20%28single-precision%29))
  ;[1 1 1] Скорость и инертность снаряда
  (Variables|/Script/Engine.MovementComponent|SetVelocity (Variables|Default|GetProjectileMovement) (* (* (Math|Vector|GetForwardVector (Variables|Default|GetSphere)) (Variables|Default|GetSpeed)) SpeedMultiplier)))

(event EventBeginPlay
  ;[1 1 1] Скорость и инертность снаряда
  (Variables|/Script/Engine.MovementComponent|SetVelocity (Variables|Default|GetProjectileMovement) (* (* (Math|Vector|GetForwardVector (Variables|Default|GetSphere)) (Variables|Default|GetSpeed)) (Variables|Default|GetSpeedMultiplier))))

(event Collision|EventHit
  (params (MyComp :type Primitive%20Component%20Object%20Reference) (Other :type Actor%20Object%20Reference) (OtherComp :type Primitive%20Component%20Object%20Reference) (bSelfMoved :type Boolean) (HitLocation :type Vector :default "0, 0, 0") (HitNormal :type Vector :default "0, 0, 0") (NormalImpulse :type Vector :default "0, 0, 0") (Hit :type Hit%20Result%20Structure%20%28by%20ref%29))
  (bind _returnvalue (Physics|IsSimulatingPhysics OtherComp "None"))
  (bind (_bblockinghit _binitialoverlap _time _distance _location _impactpoint _normal _impactnormal _physmat _hitactor _hitcomponent _hitbonename) (Collision|BreakHitResult Hit))
  (bind _returnvalue_2 (Transformation|GetWorldRotation MyComp))
  (bind _returnvalue_3 (Transformation|GetWorldTransform OtherComp))
  ;[1 1 1] Пуля
  (if (Utilities|DoesObjectImplementInterface Other "/Game/Blueprints/Weapon/BPI_TakeDamage.BPI_TakeDamage_C")
    (Class|BPITakeDamage|TakingDamage(Message) _hitactor _hitbonename 15.0 (Game|GetInstigator) "NewEnumerator0")
    (Utilities|Casting|CastToBP_Master_PlayerCharacter Other
      (:then
        _)
      (:CastFailed
        (if _returnvalue
          _
          (else
            _))))
    (else
      (if _returnvalue
        ;;[1 1 1] Придание импульса объекту, с которым столкнулась пуля
        (Physics|AddImpulseatLocation OtherComp (* (Transformation|GetVelocity) 3.0) (Transformation|GetActorLocation) "None"))
      ;;[1 1 1] Эффект столкнтвения, орстие от пули, звук попадания
      (Effects|SpawnEmitteratLocation "/Game/Assets/SciFiWeapLight/FX/Particles/P_Impact_Metal_Large_Light.P_Impact_Metal_Large_Light" _impactpoint (Class|KismetMathLibrary|NegateRotator _returnvalue_2))
      (Class|GameplayStatics|SpawnDecalAttached "/Game/Assets/Raznoe/bullet_hole_01_Mat.bullet_hole_01_Mat" "10.000000,10.000000,10.000000" OtherComp "None" (Math|Transform|InverseTransformLocation _returnvalue_3 _impactpoint) (Math|Transform|InverseTransformRotation _returnvalue_3 _returnvalue_2) "KeepRelativeOffset" 1e+01)
      (Audio|SpawnSoundatLocation "/Game/Assets/SciFiWeapLight/Sound/Rifle/Rifle_Whip_Cue.Rifle_Whip_Cue" HitLocation "0, 0, 0" 1.0 1.0 0.0 0 0)))
  (Actor|DestroyActor))

(fn ConstructionScript)