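; AI controller for enemy bots that runs the BT_Patrol behavior tree and an EQS query on BeginPlay.
; A looping 0.2-second timer distance-checks either player character class against the bot, setting or clearing focus and the Blackboard player keys.
; The same timer copies the pawn's Firing flag into IsFiring.
; Perception logic is disconnected, though the Player key still takes the perception event's Actor output.
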(event OnTargetPerceptionUpdated(AIPerception)
  (params (Actor :type Actor%20Object%20Reference) (Stimulus :type AI%20Stimulus%20Structure)))

(event Custom|OnShooting
  (bind _returnvalue (Game|Player|GetPlayerPawn 0))
  (bind _returnvalue_2 (Utilities|String|StringToName "PlayerNeardy?"))
  (bind _returnvalue_3 (Utilities|String|StringToName "Player"))
  (bind _self self)
  (bind _blackboard (Variables|Default|GetBlackboard))
  (bind _returnvalue_4 (AI|GetAIController _self))
  (Utilities|FlowControl|Sequence
    (:then_0
      ;[1 1 1] Зона открытия огня
      (Utilities|FlowControl|Sequence
        (:then_0
          (bind _asbp_big_player_character (Utilities|Casting|CastToBP_BigPlayerCharacter _returnvalue))
          (if (<= (Math|Vector|Distance(Vector) (Transformation|GetActorLocation _asbp_big_player_character) (Transformation|GetActorLocation (stale _asbp_ai_master))) 3e+03)
            (AI|Components|Blackboard|SetValueasObject _blackboard _returnvalue_3 (stale OnTargetPerceptionUpdated(AIPerception) Actor) :!label _label)
            (AI|Components|Blackboard|SetValueasBool _blackboard _returnvalue_2 true)
            (AI|SetFocus _returnvalue_4 (Game|Player|GetPlayerPawn 0))
            (else
              (AI|Components|Blackboard|ClearValue _blackboard _returnvalue_3 :!label _label_2)
              (AI|Components|Blackboard|SetValueasBool _blackboard _returnvalue_2 false)
              (AI|ClearFocus _returnvalue_4))))
        (:then_1
          (bind _asbp_master_player_character (Utilities|Casting|CastToBP_Master_PlayerCharacter _returnvalue))
          (if (<= (Math|Vector|Distance(Vector) (Transformation|GetActorLocation _asbp_master_player_character) (Transformation|GetActorLocation (stale _asbp_ai_master))) 3e+03)
            (goto _label)
            (else
              (goto _label_2))))))
    (:then_1
      ;[1 1 1] Боезапас бота
      (bind _asbp_ai_master (Utilities|Casting|CastToBP_Ai_Master (stale EventPossess PossessedPawn)))
      (AI|Components|Blackboard|SetValueasBool (Variables|Default|GetBlackboard) (Utilities|String|StringToName "IsFiring") (Variables|/Game/Blueprints/Enemy/BP_Ai_Master.BP_Ai_Master_C|GetFiring _asbp_ai_master)))))

(event EventBeginPlay
  (AI|RunBehaviorTree "/Game/Blueprints/Enemy/AI/BT_Patrol.BT_Patrol")
  (|RunEQS 0 "/Game/Blueprints/Enemy/AI/EQS_Query.EQS_Query")
  (Utilities|Time|SetTimerbyEvent (delegate Custom|OnShooting) 0.2 true))

(event EventPossess
  (params (PossessedPawn :type Pawn%20Object%20Reference))
  ;[1 1 1] Боезапас бота
)

(fn ConstructionScript)