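; Master health pickup that heals either the standard or big player character and then destroys itself.
; A timeline started on BeginPlay levitates and rotates the mesh, opening an overlap gate on update when the pickup type is Touch.
; Overlap through that gate and the interact event share one heal path, calling MedicineChest on player zero's pawn only when health is below maximum.
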(event OnComponentBeginOverlap(StaticMesh)
  (params (OverlappedComponent :type Primitive%20Component%20Object%20Reference) (OtherActor :type Actor%20Object%20Reference) (OtherComp :type Primitive%20Component%20Object%20Reference) (OtherBodyIndex :type Integer) (bFromSweep :type Boolean) (SweepResult :type Hit%20Result%20Structure%20%28by%20ref%29))
  (Utilities|FlowControl|Gate true
    (:Exit
      (|CallParentFunction)
      ;[1 1 1] Основной персонаж
      (bind _asbp_master_character (Utilities|Casting|CastToBP_Master_PlayerCharacter (Game|Player|GetPlayerPawn 0))
        (:then
          (if (not (>= (Variables|/Game/Blueprints/Player/BP_Master_PlayerCharacter.BP_Master_PlayerCharacter_C|GetCurrentHealth _asbp_master_character) (Variables|/Game/Blueprints/Player/BP_Master_PlayerCharacter.BP_Master_PlayerCharacter_C|GetMaxHealth _asbp_master_character)))
            (Default|MedicineChest _asbp_master_character (Variables|Default|GetAddHealth))
            (Actor|DestroyActor)))
        (:CastFailed
          ;[1 1 1] BidPlayer
          (bind _asbp_big_player_character (Utilities|Casting|CastToBP_BigPlayerCharacter (Game|Player|GetPlayerPawn 0)))
          (if (not (>= (Variables|/Game/MyAssets/BigPlayer/BP_BigPlayerCharacter.BP_BigPlayerCharacter_C|GetCurrentHealth _asbp_big_player_character) (Variables|/Game/MyAssets/BigPlayer/BP_BigPlayerCharacter.BP_BigPlayerCharacter_C|GetMaxHealth _asbp_big_player_character)))
            (Default|MedicineChest _asbp_big_player_character (Variables|Default|GetAddHealth))
            (Actor|DestroyActor)))))))

(event EventBeginPlay
  (bind _staticmesh (Variables|Default|GetStaticMesh))
  (|CallParentFunction)
  (bind (_direction _roatation _levitate) (Timeline|Timeline_0 Play)
    (:Update
      (Transformation|SetRelativeTransform _staticmesh (Math|Transform|MakeTransform (Math|Vector|MakeVector 0.0 0.0 _levitate) (Math|Rotator|MakeRotator 0.0 0.0 _roatation) (Transformation|GetWorldScale _staticmesh)) false false)
      (switch Utilities|FlowControl|Switch|SwitchonEnum_Interact (Variables|Default|GetType)
        (:NewEnumerator2
          (Utilities|FlowControl|Gate true) ; enters at Open
        )))))

(event EventEventInteract
  (|CallParentFunction)
  ;[1 1 1] Основной персонаж
  (bind _asbp_master_character (Utilities|Casting|CastToBP_Master_PlayerCharacter (Game|Player|GetPlayerPawn 0))
    (:then
      (if (not (>= (Variables|/Game/Blueprints/Player/BP_Master_PlayerCharacter.BP_Master_PlayerCharacter_C|GetCurrentHealth _asbp_master_character) (Variables|/Game/Blueprints/Player/BP_Master_PlayerCharacter.BP_Master_PlayerCharacter_C|GetMaxHealth _asbp_master_character)))
        (Default|MedicineChest _asbp_master_character (Variables|Default|GetAddHealth))
        (Actor|DestroyActor)))
    (:CastFailed
      ;[1 1 1] BidPlayer
      (bind _asbp_big_player_character (Utilities|Casting|CastToBP_BigPlayerCharacter (Game|Player|GetPlayerPawn 0)))
      (if (not (>= (Variables|/Game/MyAssets/BigPlayer/BP_BigPlayerCharacter.BP_BigPlayerCharacter_C|GetCurrentHealth _asbp_big_player_character) (Variables|/Game/MyAssets/BigPlayer/BP_BigPlayerCharacter.BP_BigPlayerCharacter_C|GetMaxHealth _asbp_big_player_character)))
        (Default|MedicineChest _asbp_big_player_character (Variables|Default|GetAddHealth))
        (Actor|DestroyActor)))))

(fn ConstructionScript
  (|CallParentFunction))