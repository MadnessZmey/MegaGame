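; BP_Bullet is a bullet actor that handles impact response and destroys itself on hit.
; Actors implementing BPI_TakeDamage receive damage and the hit bone, and non-simulating components also spawn a damage text actor, showing "HeadShot" for the head bone.
; Other hits spawn a metal impact particle and push simulating components with a velocity-scaled impulse.
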(event Collision|EventHit
  (params (MyComp :type Primitive%20Component%20Object%20Reference) (Other :type Actor%20Object%20Reference) (OtherComp :type Primitive%20Component%20Object%20Reference) (bSelfMoved :type Boolean) (HitLocation :type Vector :default "0, 0, 0") (HitNormal :type Vector :default "0, 0, 0") (NormalImpulse :type Vector :default "0, 0, 0") (Hit :type Hit%20Result%20Structure%20%28by%20ref%29))
  (bind _returnvalue (Physics|IsSimulatingPhysics OtherComp "None"))
  (bind (_bblockinghit _binitialoverlap _time _distance _location _impactpoint _normal _impactnormal _physmat _hitactor _hitcomponent _hitbonename) (Collision|BreakHitResult Hit))
  (bind _damage (Variables|Default|GetDamage))
  (if (Utilities|DoesObjectImplementInterface Other "/Game/Blueprints/BPI_TakeDamage.BPI_TakeDamage_C")
    (Class|BPITakeDamage|TakingDamage(Message) _hitactor _hitbonename _damage)
    (if _returnvalue
      _
      (else
        (Game|SpawnActorfromClass "/Game/UMG/BP_FloatingText.BP_FloatingText_C" (Math|Transform|MakeTransform HitLocation "0, 0, 0" "1,1,1") "Undefined" 0 (select (Utilities|Name|Equal(Name) _hitbonename "head") "HeadShot" (Utilities|Text|ToText(Float) _damage "HalfToEven" false true 1 324 0 0)) 0)))
    (else
      (if _returnvalue
        (Physics|AddImpulseatLocation OtherComp (* (Transformation|GetVelocity) 3.0) (Transformation|GetActorLocation) "None"))
      (Effects|SpawnEmitteratLocation "/Game/Assets/SciFiWeapLight/FX/Particles/P_Impact_Metal_Large_Light.P_Impact_Metal_Large_Light" _impactpoint)))
  (Actor|DestroyActor))

(fn ConstructionScript)