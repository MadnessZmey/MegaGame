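; Master weapon Blueprint for the player character, handling firing, ammo, reloading, scope zoom and flashlight/laser module switching.
; The construction script loads stats, montages and projectile class from a DT_Weapon row.
; Single, burst and auto modes use retriggerable delays for fire rate, spawning projectiles that trigger recoil and montages, with auto-reload when empty.
; Shots aim from the muzzle toward a screen-center trace hit, then receive random rotational spread.
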(event Custom|FirePress
  (params (TriggerPulled :type Boolean))
  ;[1 1 1] Стрельба и режимы стрельбы
  (Variables|Default|SetFiring TriggerPulled)
  (if (Variables|/Game/Blueprints/Player/BP_PlayerCharacter.BP_PlayerCharacter_C|GetIsFire? (Variables|Default|GetCharRef))
    (switch Utilities|FlowControl|Switch|SwitchonEnum_FireMode (Variables|Default|GetFireMode)
      (:NewEnumerator0
        (if (CallFunction|CanShoot?)
          (Variables|Default|SetFireRateDelay true)
          (CallFunction|SpawnProjectile)
          (Utilities|FlowControl|RetriggerableDelay (Variables|Default|GetFireRate))
          (Variables|Default|SetFireRateDelay false)
          (Variables|Default|SetFiring false)))
      (:NewEnumerator1
        (if (CallFunction|CanShoot?)
          (if (> (Utilities|Struct|BreakStruct_WeaponData (Variables|Default|GetWeaponData)) (Variables|Default|GetCurrentBulletsInBurst)) :!label _label
            (Variables|Default|SetFireRateDelay true)
            (Math|Integer|IncrementInt (Variables|Default|GetCurrentBulletsInBurst)
              (:%20%20
                (CallFunction|SpawnProjectile)
                (Utilities|FlowControl|RetriggerableDelay (Variables|Default|GetFireRate))
                (Variables|Default|SetFireRateDelay false)
                (goto _label)))
            (else
              (Variables|Default|SetCurrentBulletsInBurst 0)
              (Variables|Default|SetFiring false)))))
      (:NewEnumerator2
        (if (CallFunction|CanShoot?) :!label _label_2
          (Variables|Default|SetFireRateDelay true)
          (CallFunction|SpawnProjectile)
          (Utilities|FlowControl|RetriggerableDelay (Variables|Default|GetFireRate))
          (Variables|Default|SetFireRateDelay false)
          (goto _label_2))))))

(event Custom|ChangeFireMode
  ;[1 1 1] Переключение стрельбы
  (if (Utilities|Struct|BreakStruct_WeaponData (Variables|Default|GetWeaponData))
    (switch Utilities|FlowControl|Switch|SwitchonEnum_FireMode (Variables|Default|GetFireMode)
      (:NewEnumerator0
        (Variables|Default|SetFireMode "NewEnumerator1"))
      (:NewEnumerator1
        (Variables|Default|SetFireMode "NewEnumerator2" :!label _label))
      (:NewEnumerator2
        (Variables|Default|SetFireMode "NewEnumerator0" :!label _label_2)))
    (else
      (switch Utilities|FlowControl|Switch|SwitchonEnum_FireMode (Variables|Default|GetFireMode)
        (:NewEnumerator0
          (goto _label))
        (:NewEnumerator2
          (goto _label_2))))))

(event Custom|ZoomPlus
  (bind _scenecapture (Variables|Default|GetSceneCapture))
  ;[1 1 1] Изменение масштаба в прицеле
  (Variables|/Script/Engine.SceneCaptureComponent2D|SetFOVAngle _scenecapture (Math|Float|Clamp(Float) (- (Variables|/Script/Engine.SceneCaptureComponent2D|GetFOVAngle _scenecapture) 3.0) 3.0 9.0)))

(event Custom|ZoomMinus
  (bind _scenecapture (Variables|Default|GetSceneCapture))
  ;[1 1 1] Изменение масштаба в прицеле
  (Variables|/Script/Engine.SceneCaptureComponent2D|SetFOVAngle _scenecapture (Math|Float|Clamp(Float) (+ (Variables|/Script/Engine.SceneCaptureComponent2D|GetFOVAngle _scenecapture) 3.0) 3.0 9.0)))

(event Custom|AutoReload
  ;[1 1 1] Перезарядка
  ;;[1 1 1] Автоперезарядка
  (if (== (Variables|Default|GetAmmoCurrent) 0)
    (if (not (== (Variables|Default|GetAmmoMax) 0))
      (Variables|Default|SetIsReloading true)
      (CallFunction|Reloading)
      (Utilities|FlowControl|Delay (Utilities|Struct|BreakStruct_WeaponData (Variables|Default|GetWeaponData)))
      (Variables|Default|SetIsReloading false))))

(event Custom|UseModul
  (bind _laserpointer (Variables|Default|GetLaserpointer))
  (bind _flashlight (Variables|Default|GetFlashlight))
  (bind _moduleenum (Variables|Default|GetModuleEnum))
  ;[1 1 1] Переключение модулей оружия
  (Math|Integer|IncrementInt (Variables|Default|GetModuleID)
    (:%20%20
      (if (> (Variables|Default|GetModuleID) (Utilities|Array|LastIndex _moduleenum))
        (Variables|Default|SetModuleID 0))
      (switch Utilities|FlowControl|Switch|SwitchonEnum_WeaponModules (Utilities|Array|Get(acopy) _moduleenum (Variables|Default|GetModuleID))
        (:NewEnumerator0
          (Rendering|ToggleVisibility _laserpointer false))
        (:NewEnumerator1
          (Rendering|ToggleVisibility _flashlight false))
        (:NewEnumerator2
          (Rendering|ToggleVisibility _flashlight false)
          (Rendering|ToggleVisibility _laserpointer false))))))

(event Custom|ReloadWeapon
  ;[1 1 1] Перезарядка
  ;;[1 1 1] Изменение патронов при перезарядке
  (if (> (Variables|Default|GetAmmoMax) 0)
    (Variables|Default|SetNeededAmmo (- (Utilities|Struct|BreakStruct_WeaponData (Variables|Default|GetWeaponData)) (Variables|Default|GetAmmoCurrent)))
    (if (<= (Variables|Default|GetAmmoMax) (Variables|Default|GetNeededAmmo))
      (Variables|Default|SetAmmoCurrent (+ (Variables|Default|GetAmmoCurrent) (Variables|Default|GetAmmoMax)))
      (Variables|Default|SetAmmoMax 0)
      (else
        (Variables|Default|SetAmmoCurrent (Utilities|Struct|BreakStruct_WeaponData (Variables|Default|GetWeaponData)))
        (Variables|Default|SetAmmoMax (- (Variables|Default|GetAmmoMax) (Variables|Default|GetNeededAmmo)))))))

(event Custom|Reloading
  (bind _weapondata (Variables|Default|GetWeaponData))
  (bind (_reloadmontage _charreloadhip) (Utilities|Struct|BreakStruct_WeaponData _weapondata))
  ;[1 1 1] Перезарядка
  ;;[1 1 1] Ручная перезарядка
  (if (not (== (Variables|Default|GetAmmoMax) 0))
    (if (not (== (Utilities|Struct|BreakStruct_WeaponData (Variables|Default|GetWeaponData)) (Variables|Default|GetAmmoCurrent)))
      (bind _output_get (Variables|Default|SetIsReloading true))
      (if _output_get
        (CallFunction|PlayMontage _reloadmontage _charreloadhip)
        (Utilities|FlowControl|Delay (Utilities|Struct|BreakStruct_WeaponData (Variables|Default|GetWeaponData)))
        (Variables|Default|SetIsReloading false)))))

(event EventBeginPlay
  ;[1 1 1] Каст на персонажа
  (bind _asbp_player_character (Utilities|Casting|CastToBP_PlayerCharacter (Game|Player|GetPlayerPawn 0)))
  (Variables|Default|SetCharRef _asbp_player_character))

(fn ConstructionScript
  (bind _returnvalue (Utilities|GetDataTableRow "/Game/Data/DT_Weapon.DT_Weapon" (Variables|Default|GetWeaponRownName))
    (:then
      (bind _output_get (Variables|Default|SetWeaponData _returnvalue))
      (Variables|Default|SetFireMode (.FireMod (Utilities|Struct|BreakStruct_WeaponData _output_get)))
      (Variables|Default|SetMuzzleName (.MuzzleName (Utilities|Struct|BreakStruct_WeaponData _output_get)))
      (Variables|Default|SetFireRate (.FireRate (Utilities|Struct|BreakStruct_WeaponData _output_get)))
      (Variables|Default|SetReloadDelay (.ReloadDelay (Utilities|Struct|BreakStruct_WeaponData _output_get)))
      (Variables|Default|SetWeaponSpread (.WeapoSpread (Utilities|Struct|BreakStruct_WeaponData _output_get)))
      (Variables|Default|SetAmmoMax (.AmmoMax (Utilities|Struct|BreakStruct_WeaponData _output_get)))
      (Variables|Default|SetAmmoCurrent (.AmmoCurrent (Utilities|Struct|BreakStruct_WeaponData _output_get)))
      (Variables|Default|SetBulletsInShoot (.BulletsInShot (Utilities|Struct|BreakStruct_WeaponData _output_get)))
      (Variables|Default|SetProjectileClass (.ProjectileClass (Utilities|Struct|BreakStruct_WeaponData _output_get)))
      (Variables|Default|SetPlayerState (.PlayerState (Utilities|Struct|BreakStruct_WeaponData _output_get))))))

(fn CalculateDirection
  (bind _returnvalue (Game|GetPlayerController 0))
  (bind _returnvalue_2 (Viewport|GetViewportSize))
  (bind _returnvalue_3 (Utilities|MuzzlePosition))
  (bind _returnvalue_4 (/ (.y _returnvalue_2) 2.0))
  (bind _returnvalue_5 (/ (.x _returnvalue_2) 2.0))
  (bind _returnvalue_6 (Math|Vector2D|MakeVector2D _returnvalue_5 _returnvalue_4))
  (bind (_worldposition _worlddirection) (Class|GameplayStatics|DeprojectScreentoWorld _returnvalue _returnvalue_6))
  (bind _returnvalue_7 (* _worlddirection 1e+09))
  (bind (_outhit _returnvalue_8) (Collision|LineTraceByChannel _worldposition _returnvalue_7 "TraceTypeQuery1" false 0 "None"))
  (return _returnvalue_3 (Math|Rotator|FindLookatRotation _returnvalue_3 (Math|Vector|SelectVector (.ImpactPoint (Collision|BreakHitResult _outhit)) _returnvalue_7 _returnvalue_8))))

(fn SpawnProjectile
  (bind _weapondata (Variables|Default|GetWeaponData))
  (bind _weapondata_2 (Variables|Default|GetWeaponData))
  (bind (_projectilegravity _firingmontage _charfiringhip _charfiringironsight) (Utilities|Struct|BreakStruct_WeaponData _weapondata))
  (bind (_damagemin _damagemax _projectilespeed _projectilegravity_2 _damageradius) (Utilities|Struct|BreakStruct_WeaponData _weapondata_2))
  (if (CallFunction|HasAmmoinMag?)
    (CallFunction|PlayMontage _firingmontage (select (Variables|/Game/Blueprints/Player/BP_PlayerCharacter.BP_PlayerCharacter_C|GetAiming (Variables|Default|GetCharRef)) _charfiringironsight _charfiringhip))
    (for _index (range 1 (Variables|Default|GetBulletsInShoot))
      (bind (_location _rotation) (CallFunction|CalculateDirection))
      (bind _transform (CallFunction|CalculateFinalDirection _location _rotation))
      ;[1 1 1] Создание пули
      (Game|SpawnActorfromClass (Variables|Default|GetProjectileClass) _transform "Undefined" 0 _projectilespeed _projectilegravity_2 (Math|Random|RandomFloatinRange _damagemin _damagemax) _damageradius 0)
      (Default|WeaponRecoil (Variables|Default|GetCharRef) (Utilities|Struct|BreakStruct_WeaponData (Variables|Default|GetWeaponData))))
    (Math|Integer|DecrementInt (Variables|Default|GetAmmoCurrent))
    (else
      (CallFunction|AutoReload))))

(fn CalculateFinalDirection
  (params (Location :type Vector) (Rotation :type Rotator))
  (bind _weaponspread (Variables|Default|GetWeaponSpread))
  (bind _returnvalue (* _weaponspread -1.0))
  ;[1 1 1] Разброс пуль
  (return (Math|Transform|MakeTransform Location (Math|Rotator|CombineRotators Rotation (Math|Rotator|MakeRotator (Math|Random|RandomFloatinRange _returnvalue _weaponspread) (Math|Random|RandomFloatinRange _returnvalue _weaponspread) (Math|Random|RandomFloatinRange _returnvalue _weaponspread))))))

(fn PlayMontage
  (params (WeaponAnim :type Anim%20Montage%20Object%20Reference) (CharAnim :type Anim%20Montage%20Object%20Reference))
  ;[1 1 1] Анимация оружия при стельбе
  (Animation|Montage|MontagePlay (Components|SkeletalMesh|GetAnimInstance (Variables|Default|GetWeaponMesh)) WeaponAnim 1.0 "MontageLength" 0.0 true)
  ;[1 1 1] Анимация персонажа (отдача)
  (Animation|Montage|MontagePlay (Components|SkeletalMesh|GetAnimInstance (Variables|/Script/Engine.Character|GetMesh (Variables|Default|GetCharRef))) CharAnim 1.0 "MontageLength" 0.0 true))

(fn HasAmmoinMag?
  (return (> (Variables|Default|GetAmmoCurrent) 0)))

(fn CanShoot?
  (return (Math|Boolean|ANDBoolean (Variables|Default|GetFiring) (not (Variables|Default|GetIsReloading)) (not (Variables|Default|GetFireRateDelay)))))