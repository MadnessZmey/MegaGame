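; Base weapon projectile that launches along its sphere's forward vector with configurable speed and gravity; SwitchSpeed re-applies velocity with a multiplier.
; On hit it branches on Type, then destroys itself.
; Bullets send bone-specific damage through BPI_TakeDamage, or else push physics objects and spawn impact particles, attached decal and sound.
; Rockets spawn explosion effects and apply radial damage.
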(event Custom|SwitchSpeed
  (params (SpeedMultiplier :type Float%20%28single-precision%29))
  ;[1 1 1] Скорость и инертность снаряда
  (Variables|/Script/Engine.MovementComponent|SetVelocity (Variables|Default|GetProjectileMovement) (* (* (Math|Vector|GetForwardVector (Variables|Default|GetSphere)) (Variables|Default|GetSpeed)) SpeedMultiplier)))

(event EventBeginPlay
  ;[1 1 1] Скорость и инертность снаряда
  (Variables|/Script/Engine.MovementComponent|SetVelocity (Variables|Default|GetProjectileMovement) (* (* (Math|Vector|GetForwardVector (Variables|Default|GetSphere)) (Variables|Default|GetSpeed)) (Variables|Default|GetSpeedMultiplier)))
  (Variables|/Script/Engine.ProjectileMovementComponent|SetProjectileGravityScale (Variables|Default|GetProjectileMovement) (Variables|Default|GetGravity)))

(event Collision|EventHit
  (params (MyComp :type Primitive%20Component%20Object%20Reference) (Other :type Actor%20Object%20Reference) (OtherComp :type Primitive%20Component%20Object%20Reference) (bSelfMoved :type Boolean) (HitLocation :type Vector :default "0, 0, 0") (HitNormal :type Vector :default "0, 0, 0") (NormalImpulse :type Vector :default "0, 0, 0") (Hit :type Hit%20Result%20Structure%20%28by%20ref%29))
  (bind (_bblockinghit _binitialoverlap _time _distance _location _impactpoint _normal _impactnormal _physmat _hitactor _hitcomponent _hitbonename) (Collision|BreakHitResult Hit))
  (bind (_x _y _z) (Math|Vector|BreakVector HitLocation))
  (bind _returnvalue (Transformation|GetWorldRotation MyComp))
  (bind _returnvalue_2 (Transformation|GetWorldTransform OtherComp))
  (switch Utilities|FlowControl|Switch|SwitchonEnum_ProjectileType (Variables|Default|GetType)
    (:NewEnumerator0
      ;[1 1 1] Пуля
      (if (Utilities|DoesObjectImplementInterface Other "/Game/Blueprints/Weapon/BPI_TakeDamage.BPI_TakeDamage_C")
        (Class|BPITakeDamage|TakingDamage(Message) _hitactor _hitbonename (Variables|Default|GetDamage) (Game|GetInstigator) "NewEnumerator0")
        (else
          (if (Physics|IsSimulatingPhysics OtherComp "None")
            ;;[1 1 1] Придание импульса объекту, с которым столкнулась пуля
            (Physics|AddImpulseatLocation OtherComp (* (Transformation|GetVelocity) 3.0) (Transformation|GetActorLocation) "None"))
          ;;[1 1 1] Эффект столкнтвения, орстие от пули, звук попадания
          (Effects|SpawnEmitteratLocation "/Game/Assets/SciFiWeapLight/FX/Particles/P_Impact_Metal_Large_Light.P_Impact_Metal_Large_Light" _impactpoint (Class|KismetMathLibrary|NegateRotator _returnvalue))
          (Class|GameplayStatics|SpawnDecalAttached "/Game/Assets/Raznoe/bullet_hole_01_Mat.bullet_hole_01_Mat" "10.000000,10.000000,10.000000" OtherComp "None" (Math|Transform|InverseTransformLocation _returnvalue_2 _impactpoint) (Math|Transform|InverseTransformRotation _returnvalue_2 _returnvalue) "KeepRelativeOffset" 1e+01)
          (Audio|SpawnSoundatLocation "/Game/Assets/SciFiWeapLight/Sound/Rifle/Rifle_Whip_Cue.Rifle_Whip_Cue" _impactpoint "0, 0, 0" 1.0 1.0 0.0 0 0)))
      (Actor|DestroyActor))
    (:NewEnumerator1
      ;[1 1 1] Рокета
      (Effects|SpawnEmitteratLocation "/Game/Assets/SciFiWeapLight/FX/Particles/P_RocketLauncher_Explosion_Light.P_RocketLauncher_Explosion_Light" HitLocation)
      (Audio|SpawnSoundatLocation "/Game/Assets/SciFiWeapLight/Sound/RocketLauncher/RL_Explosion_Cue.RL_Explosion_Cue" HitLocation "0, 0, 0" 1.0 1.0 0.0 0 0)
      (Game|Damage|ApplyRadialDamage (Variables|Default|GetDamage) (Math|Vector|MakeVector _x _y (+ _z 1e+01)) (Variables|Default|GetDamageRadius) 0 0 0 0 false "ECC_Visibility")
      (Actor|DestroyActor))))

(fn ConstructionScript)