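; BP_Zone is a battle royale zone actor that flags player characters as they enter or leave its cube volume.
; On BeginPlay the Size_1 timeline animates the cube's X scale, and a 15-second Delay on its update leads into the Size_2 timeline for a second resize.
; Overlap begin sets Outside to true on BP_PlayerCharacter and overlap end clears it, so the cube itself counts as the outside area.
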(event OnComponentBeginOverlap(Cube)
  (params (OverlappedComponent :type Primitive%20Component%20Object%20Reference) (OtherActor :type Actor%20Object%20Reference) (OtherComp :type Primitive%20Component%20Object%20Reference) (OtherBodyIndex :type Integer) (bFromSweep :type Boolean) (SweepResult :type Hit%20Result%20Structure%20%28by%20ref%29))
  (bind _asbp_player_character (Utilities|Casting|CastToBP_PlayerCharacter OtherActor))
  (Variables|/Game/Blueprints/Player/BP_PlayerCharacter.BP_PlayerCharacter_C|SetOutside _asbp_player_character true))

(event OnComponentEndOverlap(Cube)
  (params (OverlappedComponent :type Primitive%20Component%20Object%20Reference) (OtherActor :type Actor%20Object%20Reference) (OtherComp :type Primitive%20Component%20Object%20Reference) (OtherBodyIndex :type Integer))
  (bind _asbp_player_character (Utilities|Casting|CastToBP_PlayerCharacter OtherActor))
  (Variables|/Game/Blueprints/Player/BP_PlayerCharacter.BP_PlayerCharacter_C|SetOutside _asbp_player_character false))

(event EventBeginPlay
  (bind _t_zone1 (Timeline|Size_1 Play)
    (:Update
      (Transformation|SetWorldScale3D (Variables|Default|GetCube) (Math|Vector|MakeVector (.x (Math|Conversions|ToVector(Float) _t_zone1)) 1e+01 1e+01))
      (Utilities|FlowControl|Delay 15.0)
      (bind _t_zone2 (Timeline|Size_2 Play)
        (:Update
          (Transformation|SetWorldScale3D (Variables|Default|GetCube) (Math|Vector|MakeVector (.x (Math|Conversions|ToVector(Float) _t_zone2)) 1e+01 1e+01)))))))

(fn ConstructionScript)